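; Boxing-glove obstacle for the Boxing Jumps racing minigame that punches players away.
; BeginPlay runs an endless delay loop alternating two timelines: one slides the middle glove (Glove1) along local Y, the other slides Scene1.
; Glove overlaps call getPunched, which launches BP_PlayerMaster along fixed world -Y with slight lift, only while the checked component is displaced from rest.
; The other two gloves both check Scene1's offset.
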(event OnComponentBeginOverlap(BoxingJumps_Boxing_Glove)
  (params (OverlappedComponent :type Primitive%20Component%20Object%20Reference) (OtherActor :type Actor%20Object%20Reference) (OtherComp :type Primitive%20Component%20Object%20Reference) (OtherBodyIndex :type Integer) (bFromSweep :type Boolean) (SweepResult :type Hit%20Result%20Structure%20%28by%20ref%29))
  (CallFunction|GetPunched OtherActor (Variables|/Script/Engine.SceneComponent|GetRelativeLocation (Variables|Default|GetScene1))))

(event OnComponentBeginOverlap(BoxingJumps_Boxing_Glove1)
  (params (OverlappedComponent :type Primitive%20Component%20Object%20Reference) (OtherActor :type Actor%20Object%20Reference) (OtherComp :type Primitive%20Component%20Object%20Reference) (OtherBodyIndex :type Integer) (bFromSweep :type Boolean) (SweepResult :type Hit%20Result%20Structure%20%28by%20ref%29))
  (CallFunction|GetPunched OtherActor (Variables|/Script/Engine.SceneComponent|GetRelativeLocation (Variables|Default|GetBoxingJumps_Boxing_Glove1))))

(event OnComponentBeginOverlap(BoxingJumps_Boxing_Glove2)
  (params (OverlappedComponent :type Primitive%20Component%20Object%20Reference) (OtherActor :type Actor%20Object%20Reference) (OtherComp :type Primitive%20Component%20Object%20Reference) (OtherBodyIndex :type Integer) (bFromSweep :type Boolean) (SweepResult :type Hit%20Result%20Structure%20%28by%20ref%29))
  (CallFunction|GetPunched OtherActor (Variables|/Script/Engine.SceneComponent|GetRelativeLocation (Variables|Default|GetScene1))))

(event Custom|Punch2
  (bind _alpha (Timeline|Timeline_0 PlayFromStart)
    (:Update
      (Transformation|SetRelativeLocation (Variables|Default|GetScene1) (Math|Vector|MakeVector 0.0 (Math|Float|Lerp 0.0 -1e+02 _alpha) 0.0) false false))))

(event Custom|Punch
  (bind _boxingjumps_boxing_glove1 (Variables|Default|GetBoxingJumps_Boxing_Glove1))
  (bind _relativelocation (Variables|/Script/Engine.SceneComponent|GetRelativeLocation _boxingjumps_boxing_glove1))
  (bind _alpha (Timeline|PunchT PlayFromStart)
    (:Update
      (Transformation|SetRelativeLocation _boxingjumps_boxing_glove1 (Math|Vector|MakeVector (.x _relativelocation) (Math|Float|Lerp 0.0 -1e+02 _alpha) (.z _relativelocation)) false false))))

(event Custom|getPunched
  (params (NewParam :type Actor%20Object%20Reference) (A :type Vector))
  (bind _asbp_player_master (Utilities|Casting|CastToBP_PlayerMaster NewParam))
  (if (< (.y A) -1.0)
    (Character|LaunchCharacter _asbp_player_master "0.000000,-2000.000000,200.000000" false false)))

(event EventBeginPlay
  (bind _punchdelay (Variables|Default|GetPunchDelay))
  (CallFunction|Punch :!label _label)
  (Utilities|FlowControl|Delay _punchdelay)
  (CallFunction|Punch2)
  (Utilities|FlowControl|Delay _punchdelay)
  (goto _label))

(event Collision|EventActorBeginOverlap
  (params (OtherActor :type Actor%20Object%20Reference)))

(fn ConstructionScript)