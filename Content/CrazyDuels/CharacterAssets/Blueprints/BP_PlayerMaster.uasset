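; Base player character for CrazyDuels, with camera-relative movement, look, jump, slide and death.
; BeginPlay layers physical animation with simulated physics below two configurable bones, and Die extends it from the hips while disabling movement.
; Slide raises speed and plays the Glide timeline to cut friction, shrink the capsule and adjust the Scene component's transform, blocking walk input after a short delay until release reverses it.
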(event Custom|Die
  (bind _returnvalue (Utilities|Name|MakeLiteralName "Hips"))
  (Class|SkeletalMeshComponent|SetAllBodiesBelowSimulatePhysics (Variables|Default|GetSkeletalMesh) _returnvalue true true)
  (Class|PhysicalAnimationComponent|ApplyPhysicalAnimationSettingsBelow (Variables|Default|GetPhysicalAnimation) _returnvalue (Utilities|Struct|MakePhysicalAnimationData true 2e+02 2e+02 1e+03 1e+02) true)
  (Pawn|Components|CharacterMovement|DisableMovement (Variables|Character|GetCharacterMovement)))

(event EventBeginPlay
  (bind _bonephysics1 (Variables|Default|GetBonePhysics1))
  (bind _skeletalmesh (Variables|Default|GetSkeletalMesh))
  (bind _bonephysics2 (Variables|Default|GetBonePhysics2))
  (bind _physicalanimation (Variables|Default|GetPhysicalAnimation))
  (Class|PhysicalAnimationComponent|SetSkeletalMeshComponent _physicalanimation _skeletalmesh)
  (Class|PhysicalAnimationComponent|ApplyPhysicalAnimationSettingsBelow _physicalanimation _bonephysics2 (Utilities|Struct|MakePhysicalAnimationData true 1e+02 1e+02 1e+03 1e+02) true)
  (Class|SkeletalMeshComponent|SetAllBodiesBelowSimulatePhysics _skeletalmesh _bonephysics2 true true)
  (Class|PhysicalAnimationComponent|ApplyPhysicalAnimationSettingsBelow _physicalanimation _bonephysics1 (Utilities|Struct|MakePhysicalAnimationData true 1e+02 1e+02 1e+03 1e+02) true)
  (Class|SkeletalMeshComponent|SetAllBodiesBelowSimulatePhysics _skeletalmesh _bonephysics1 true true))

(event Input|ActionEvents|InputActionJump
  (params (Key :type Key%20Structure :default "None"))
  (:Pressed
    (Character|Jump)))

(event Input|ActionEvents|InputActionSlide
  (params (Key :type Key%20Structure :default "None"))
  (bind _charactermovement (Variables|Character|GetCharacterMovement))
  (bind _charactermovement_2 (Variables|Character|GetCharacterMovement))
  (:Pressed
    (Utilities|FlowControl|Sequence
      (:then_0
        (Variables|/Script/Engine.CharacterMovementComponent|SetMaxWalkSpeed _charactermovement 1e+03)
        (bind _alpha (Timeline|Glide Play)
          (:Update
            (Transformation|SetRelativeRotation (Variables|Default|GetScene) (Math|Rotator|Lerp(Rotator) "0, 0, 0" "0, 0,90.000000" _alpha true) false false)
            (Variables|/Script/Engine.CharacterMovementComponent|SetGroundFriction _charactermovement_2 (Math|Float|Lerp 8.0 0.0 _alpha))
            (Variables|/Script/Engine.CharacterMovementComponent|SetBrakingFriction _charactermovement_2 (Math|Float|Lerp 2.0 0.0 _alpha))
            (Components|Capsule|SetCapsuleHalfHeight (Variables|Collision|GetCapsuleComponent) (Math|Float|Lerp 88.0 34.0 _alpha) true)
            (Transformation|SetRelativeLocation (Variables|Default|GetScene) (Math|Vector|Lerp(Vector) "0, 0,60.000000" "0, 0,160.000000" _alpha) false false))))
      (:then_1
        (Utilities|FlowControl|RetriggerableDelay 0.2)
        (Variables|Default|SetCanWalk false))))
  (:Released
    (Variables|/Script/Engine.CharacterMovementComponent|SetMaxWalkSpeed _charactermovement 5e+02)
    (Variables|Default|SetCanWalk true)
    (Timeline|Glide Reverse)))

(event Input|AxisEvents|InputAxisMoveForward
  (params (AxisValue :type Float%20%28single-precision%29))
  ;[1 1 1] Movement
  (if (Variables|Default|GetCanWalk)
    (Pawn|Input|AddMovementInput (Math|Vector|GetForwardVector (Math|Rotator|MakeRotator 0.0 0.0 (.yaw (Pawn|GetControlRotation :!class /Script/Engine.Pawn)))) AxisValue false)))

(event Input|AxisEvents|InputAxisMoveRight
  (params (AxisValue :type Float%20%28single-precision%29))
  ;[1 1 1] Movement
  (if (Variables|Default|GetCanWalk)
    (Pawn|Input|AddMovementInput (Math|Vector|GetRightVector (Math|Rotator|MakeRotator 0.0 0.0 (.yaw (Pawn|GetControlRotation :!class /Script/Engine.Pawn)))) AxisValue false)))

(event Input|AxisEvents|InputAxisLookUp
  (params (AxisValue :type Float%20%28single-precision%29))
  ;[1 1 1] CameraRotation
  (Pawn|Input|AddControllerPitchInput AxisValue))

(event Input|AxisEvents|InputAxisTurn
  (params (AxisValue :type Float%20%28single-precision%29))
  ;[1 1 1] CameraRotation
  (Pawn|Input|AddControllerYawInput AxisValue))

(event Input|AxisEvents|InputAxisTurnRate
  (params (AxisValue :type Float%20%28single-precision%29))
  (Pawn|Input|AddControllerYawInput (* AxisValue 0.4)))

(event Input|AxisEvents|InputAxisLookUpRate
  (params (AxisValue :type Float%20%28single-precision%29))
  (Pawn|Input|AddControllerPitchInput (* AxisValue 0.4)))

(fn ConstructionScript)